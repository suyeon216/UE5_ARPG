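; PC_PlayerController is the player controller that relays player stat changes to the HUD and limits camera pitch.
; On possessing a BP_Player, it binds handlers to that pawn's HP and stamina change events.
; Each handler casts player 0's HUD to Hud_Main and forwards the values to its UIPlay widget.
; BeginPlay narrows the camera manager's view pitch range; Tick is empty, and an IsAlive message check is left disconnected.
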(event `self.ReceivePossess`
  (params (PossessedPawn :type "Pawn Object Reference"))
  (bind _asbp_player (cast `/Game/BluePrint/BP_Player` PossessedPawn))
  (add `/Game/BluePrint/BP_Player.HpChange` _asbp_player (delegate `OnHpChange`))
  (add `/Game/BluePrint/BP_Player.StaminaChange` _asbp_player (delegate `OnStaminaChange`)))

(event `OnHpChange`
  (params (Hp :type "Float (double-precision)") (MaxHp :type "Float (double-precision)"))
  (bind _ashud_main (cast `/Game/Framework/Hud_Main` (`self.GetHUD` (`GameplayStatics.GetPlayerController` 0))))
  (`/Engine/EditorBlueprintResources/StandardMacros.IsValid` _ashud_main
    (:`Is Valid`
      (`/Game/UI/WBP_PlayUI.OnHpChange` (`/Game/Framework/Hud_Main.UI_Play` _ashud_main) Hp MaxHp))))

(event `OnStaminaChange`
  (params (Stamina :type "Float (double-precision)") (MaxStamina :type "Float (double-precision)"))
  (bind _ashud_main (cast `/Game/Framework/Hud_Main` (`self.GetHUD` (`GameplayStatics.GetPlayerController` 0))))
  (`/Engine/EditorBlueprintResources/StandardMacros.IsValid` _ashud_main
    (:`Is Valid`
      (`/Game/UI/WBP_PlayUI.OnStaminaChange` (`/Game/Framework/Hud_Main.UI_Play` _ashud_main) Stamina MaxStamina))))

(event `self.ReceiveBeginPlay`
  (bind _returnvalue (`GameplayStatics.GetPlayerCameraManager` 0))
  (set `PlayerCameraManager.ViewPitchMin` -40.0 _returnvalue)
  (set `PlayerCameraManager.ViewPitchMax` 30.0 _returnvalue))

(event `self.ReceiveTick`
  (params (DeltaSeconds :type "Float (single-precision)")))

(fn `UserConstructionScript`)