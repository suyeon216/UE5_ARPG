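; Base enemy Blueprint that chases the player, returns to its spawn point, takes damage and dies as a ragdoll.
; A self-recalling delayed loop scans SphereSearch for the Player tag, using a forward dot-product test to choose AI MoveTo toward player or home.
; Damage has a brief invulnerability window, and death enables physics before delayed destruction.
; AttackCheck overlaps only toggle CanAttack; no attack logic runs here.
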(event `self.ReceiveBeginPlay`
  (set `self.BeginLocation` (`self.K2_GetActorLocation`))
  (set `self.BeginRotation` (`self.K2_GetActorRotation`))
  (`self.FindPlayerAndMove`))

(event `self.ReceiveAnyDamage`
  (params (Damage :type "Float (single-precision)") (DamageType :type "DamageType Object Reference") (InstigatedBy :type "Controller Object Reference") (DamageCauser :type "Actor Object Reference"))
  ; 받는 데미지 처리
  (if (not (`self.IsGetDamage`))
    (bind _output_get (set `self.Hp` (- (`self.Hp`) Damage)))
    (set `self.IsGetDamage` true)
    (`|ExecutionSequence`
      (:`then_0`
        (if (<= _output_get 0.0)
          (`self.OnDie`)))
      (:`then_1`
        (`KismetSystemLibrary.Delay` 0.3)
        (set `self.IsGetDamage` false)))))

(event `OnDie`
  (bind _mesh (`self.Mesh`))
  ; Die 기능
  (`PrimitiveComponent.SetCollisionProfileName` _mesh "Ragdoll" false)
  (`PrimitiveComponent.SetSimulatePhysics` _mesh true)
  (`KismetSystemLibrary.Delay` 5.0)
  (`self.K2_DestroyActor`))

(event `FindPlayerAndMove`
  (bind _player (`self.Player`))
  ; 플레이어 탐색 후 찾으면 플레이어한테 이동
  (if (`self.CanMove`)
    (set `self.IsInPlayer` false)
    (`KismetSystemLibrary.Delay` 0.1)
    (for _array_element (`PrimitiveComponent.GetOverlappingComponents` (`self.Sphere_Search`))
      (if (`ActorComponent.ComponentHasTag` _array_element "Player")
        (set `self.IsInPlayer` true)
        (set `self.Player` (`ActorComponent.GetOwner` _array_element))
        (break)))
    (`/Engine/EditorBlueprintResources/StandardMacros.IsValid` _player
      (:`Is Valid`
        (if (and (`self.IsInPlayer`) (< (`KismetMathLibrary.Dot_VectorVector` (- (`self.K2_GetActorLocation`) (`self.K2_GetActorLocation` _player)) (`self.GetActorForwardVector`)) 70.0))
          (`|AIMoveTo` self (0.0 0.0 0.0) (`self.Player`) 100.0
            (:`then`
              (set `self.IsMove` true :!label _label))
            (:`OnSuccess`
              (set `self.IsMove` false))
            (:`OnFail`
              (goto _label)))
          (else
            (`|AIMoveTo` self (`self.BeginLocation`) null 100.0 :!label _label_2
              (:`then`
                (set `self.IsMove` true :!label _label_3))
              (:`OnSuccess`
                (set `self.IsMove` false)
                (`self.K2_SetActorRotation` (`self.BeginRotation`)))
              (:`OnFail`
                (goto _label_3))))))
      (:`Is Not Valid`
        (goto _label_2)))
    (`self.FindPlayerAndMove`)
    (else
      (`KismetSystemLibrary.Delay` 0.2)
      (`self.FindPlayerAndMove`))))

(event `self.AttackCheck.OnComponentBeginOverlap`
  (params (OverlappedComponent :type "PrimitiveComponent Object Reference") (OtherActor :type "Actor Object Reference") (OtherComp :type "PrimitiveComponent Object Reference") (OtherBodyIndex :type Integer) (bFromSweep :type Boolean) (SweepResult :type "HitResult Structure (by ref)"))
  ; 공격범위 안에 있는지 검사
  (if (`ActorComponent.ComponentHasTag` OtherComp "Player")
    (set `self.CanAttack` true)))

(event `self.AttackCheck.OnComponentEndOverlap`
  (params (OverlappedComponent :type "PrimitiveComponent Object Reference") (OtherActor :type "Actor Object Reference") (OtherComp :type "PrimitiveComponent Object Reference") (OtherBodyIndex :type Integer))
  ; 공격범위 안에 있는지 검사
  (if (`ActorComponent.ComponentHasTag` OtherComp "Player")
    (set `self.CanAttack` false)))

(fn `UserConstructionScript`)