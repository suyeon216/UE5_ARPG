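; Child enemy Blueprint for a sword-and-shield melee attacker that repeatedly swings and damages components tagged Player.
; BeginPlay sets health and power, then starts a self-calling Attack loop that polls CanAttack, locks movement and resumes after EndAttackMotion.
; StartAttack and EndAttack toggle sword collision, whose overlaps apply Power as damage.
; OnDie turns off sword and shield overlaps and capsule collision before calling the parent.
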(event `self.ReceiveBeginPlay`
  (`parent.ReceiveBeginPlay`)
  (set `self.Hp` 100.0)
  (`self.Attack`)
  (set `self.Power` 10.0))

(event `self.ReceiveTick`
  (params (DeltaSeconds :type "Float (single-precision)"))
  (`parent.ReceiveTick` DeltaSeconds))

(event `Attack`
  (if (`self.CanAttack`)
    (set `self.IsAttack` true)
    (set `self.CanMove` false)
    (else
      (`KismetSystemLibrary.Delay` 0.2)
      (`self.Attack`))))

(event `/Game/Interface/BPI_PlayerData.StartAttack`
  (`PrimitiveComponent.SetCollisionEnabled` (`self.SwordColl`) "QueryOnly"))

(event `/Game/Interface/BPI_PlayerData.EndAttack`
  (`PrimitiveComponent.SetCollisionEnabled` (`self.SwordColl`) "NoCollision"))

(event `/Game/Interface/BPI_PlayerData.EndAttackMotion`
  (set `self.CanMove` true)
  (set `self.IsAttack` false)
  (`KismetSystemLibrary.Delay` 0.2)
  (set `self.CanAttack` true)
  (`self.Attack`))

(event `self.SwordColl.OnComponentBeginOverlap`
  (params (OverlappedComponent :type "PrimitiveComponent Object Reference") (OtherActor :type "Actor Object Reference") (OtherComp :type "PrimitiveComponent Object Reference") (OtherBodyIndex :type Integer) (bFromSweep :type Boolean) (SweepResult :type "HitResult Structure (by ref)"))
  (if (not (== (`ActorComponent.ComponentHasTag` OtherComp "Player") (== OtherActor self)))
    (`KismetSystemLibrary.PrintString` (`KismetSystemLibrary.GetObjectName` OtherComp))
    (`GameplayStatics.ApplyDamage` OtherActor (`self.Power`))))

(event `self.OnDie`
  (set `PrimitiveComponent.bGenerateOverlapEvents` false (`self.SwordColl`))
  (set `PrimitiveComponent.bGenerateOverlapEvents` false (`self.ShieldColl`))
  (`PrimitiveComponent.SetCollisionEnabled` (`self.CapsuleComponent`) "NoCollision")
  (`parent.OnDie`))

(fn `UserConstructionScript`
  (`parent.UserConstructionScript`))