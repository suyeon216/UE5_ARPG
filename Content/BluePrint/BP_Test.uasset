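; BP_Test is a test melee character with move, look, sprint, block and health logic.
; Sprint input drains stamina to raise walk speed, while movement is gated on attacking or blocking.
; Tick restarts a one-second attack whenever none is running, enabling the sword collider that applies Power as damage on overlap.
; Blocking enables the shield collider and negates incoming damage; otherwise Hp drops, and death switches the mesh to ragdoll.
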(event `self.ReceiveBeginPlay`
  (set `self.Stamina` (`self.MaxStamina`)))

(event `EnhancedInput|/Game/Input/IA_PlayerMove`
  (params (ActionValue :type "Vector2D Structure") (ElapsedSeconds :type "Float (double-precision)") (TriggeredSeconds :type "Float (double-precision)") (InputAction :type "InputAction Object Reference" :default "/Game/Input/IA_PlayerMove.IA_PlayerMove"))
  (bind (_returnvalue_roll _returnvalue_pitch _returnvalue_yaw) (`KismetMathLibrary.BreakRotator` (`self.GetControlRotation`)))
  (bind (_returnvalue_x _returnvalue_y) (`KismetMathLibrary.BreakVector2D` (`KismetMathLibrary.Normal2D` ActionValue)))
  (bind _returnvalue (`KismetMathLibrary.MakeRotator` 0.0 0.0 _returnvalue_yaw))
  (:`Triggered`
    (bind _iscanmove (`self.IsCanMove`))
    (if _iscanmove
      (`self.AddMovementInput` (`KismetMathLibrary.GetRightVector` _returnvalue) _returnvalue_x)
      (`self.AddMovementInput` (`KismetMathLibrary.GetForwardVector` _returnvalue) _returnvalue_y))))

(event `EnhancedInput|/Game/Input/IA_BPlayerAction`
  (params (ActionValue :type Boolean) (ElapsedSeconds :type "Float (double-precision)") (TriggeredSeconds :type "Float (double-precision)") (InputAction :type "InputAction Object Reference" :default "/Game/Input/IA_BPlayerAction.IA_BPlayerAction"))
  (bind _charactermovement (`self.CharacterMovement`))
  (:`Triggered`
    (if ActionValue
      (bind _iscanusestamina (`self.IsCanUseStamina` 1.0 :!label _label))
      (if _iscanusestamina
        (bind _output_get (set `self.MoveSpeed` 600.0))
        (set `CharacterMovementComponent.MaxWalkSpeed` _output_get _charactermovement)
        (else
          (bind _output_get_2 (set `self.MoveSpeed` 400.0 :!label _label_2))
          (set `CharacterMovementComponent.MaxWalkSpeed` _output_get_2 _charactermovement)))
      (else
        (goto _label_2))))
  (:`Ongoing`
    (goto _label))
  (:`Completed`
    (goto _label_2)))

(event `EnhancedInput|/Game/Input/IA_PlayerLook`
  (params (ActionValue :type "Vector2D Structure") (ElapsedSeconds :type "Float (double-precision)") (TriggeredSeconds :type "Float (double-precision)") (InputAction :type "InputAction Object Reference" :default "/Game/Input/IA_PlayerLook.IA_PlayerLook"))
  (bind (_returnvalue_x _returnvalue_y) (`KismetMathLibrary.BreakVector2D` (* ActionValue (`self.MouseSensitivity`))))
  (:`Triggered`
    (`self.AddControllerYawInput` _returnvalue_x)
    (`self.AddControllerPitchInput` _returnvalue_y)))

(event `self.ReceiveTick`
  (params (DeltaSeconds :type "Float (single-precision)"))
  (if (not (`self.IsAttack`))
    (`self.Attack`)))

(event `Attack`
  (bind _swordcollision (`self.SwordCollision`))
  (`PrimitiveComponent.SetCollisionEnabled` _swordcollision "QueryOnly")
  (set `self.IsAttack` true)
  (`KismetSystemLibrary.Delay` 1.0)
  (`PrimitiveComponent.SetCollisionEnabled` _swordcollision "NoCollision")
  (set `self.IsAttack` false))

(event `EnhancedInput|/Game/Input/IA_PlayerBlock`
  (params (ActionValue :type Boolean) (ElapsedSeconds :type "Float (double-precision)") (TriggeredSeconds :type "Float (double-precision)") (InputAction :type "InputAction Object Reference" :default "/Game/Input/IA_PlayerBlock.IA_PlayerBlock"))
  (:`Triggered`
    (if (not (`self.IsAttack`))
      (set `self.IsBlock` ActionValue)
      (`PrimitiveComponent.SetCollisionEnabled` (`self.ShieldCollision`) "QueryOnly"))))

(event `NotBlock`
  (set `self.IsBlock` false)
  (`PrimitiveComponent.SetCollisionEnabled` (`self.ShieldCollision`) "NoCollision"))

(event `self.SwordCollision.OnComponentBeginOverlap`
  (params (OverlappedComponent :type "PrimitiveComponent Object Reference") (OtherActor :type "Actor Object Reference") (OtherComp :type "PrimitiveComponent Object Reference") (OtherBodyIndex :type Integer) (bFromSweep :type Boolean) (SweepResult :type "HitResult Structure (by ref)"))
  (if (`ActorComponent.ComponentHasTag` OtherComp "CameraTrigger")
    _
    (elif (not (== OtherActor self))
      (`GameplayStatics.ApplyDamage` OtherActor (`self.Power`)))))

(event `self.ReceiveAnyDamage`
  (params (Damage :type "Float (single-precision)") (DamageType :type "DamageType Object Reference") (InstigatedBy :type "Controller Object Reference") (DamageCauser :type "Actor Object Reference"))
  (if (`self.IsBlock`)
    (`KismetSystemLibrary.PrintString` "Block")
    (else
      (bind _output_get (set `self.Hp` (- (`self.Hp`) Damage)))
      (if (<= _output_get 0.0)
        (`self.OnDie`)))))

(event `OnDie`
  (bind _mesh (`self.Mesh`))
  (`PrimitiveComponent.SetCollisionProfileName` _mesh "Ragdoll" false)
  (`PrimitiveComponent.SetSimulatePhysics` _mesh true))

(fn `IsAlive`
  (returns (IsAlive :type Boolean))
  (return (> (`self.Hp`) 0.0)))

(fn `IsCanMove`
  (returns (IsCanMove :type Boolean))
  (return (not (or (`self.IsAttack`) (`self.IsBlock`)))))

(fn `IsCanUseStamina`
  (params (UseStamina :type "Float (double-precision)"))
  (returns (IsCanUseStamina :type Boolean))
  (bind _returnvalue (- (`self.Stamina`) UseStamina))
  (bind _returnvalue_2 (> _returnvalue 0.0))
  (if _returnvalue_2
    (bind _output_get (set `self.Stamina` _returnvalue))
    (`self.StaminaChange` _output_get (`self.MaxStamina`)))
  (return _returnvalue_2))

(fn `UserConstructionScript`
  (set `CharacterMovementComponent.MaxWalkSpeed` (`self.MoveSpeed`) (`self.CharacterMovement`)))