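; Player character for melee combat, with Enhanced Input movement, sprint, sword attacks, shield blocking and target lock-on.
; A shared stamina pool pays for sprinting, attacking and blocked damage, regenerates outside attack and block, and reports changes alongside HP.
; Start/end attack events toggle sword collision for overlap damage, while lock-on faces the nearest actor tracked by a sphere.
; Death unpossesses, ragdolls, notifies the GameMode for respawn and destroys the actor.
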(event `self.ReceiveBeginPlay`
  (`EnhancedInputSubsystemInterface.AddMappingContext` (pcsubsystem `EnhancedInputLocalPlayerSubsystem` (`GameplayStatics.GetPlayerController` 0)) "/Game/Input/IAC_Player.IAC_Player" 0 (struct))
  (set `self.Stamina` (`self.MaxStamina`))
  (`self.HpChange` (`self.Hp`) (`self.MaxHp`))
  (`self.StaminaChange` (`self.Stamina`) (`self.MaxStamina`)))

(event `EnhancedInput|/Game/Input/IA_PlayerMove`
  (params (ActionValue :type "Vector2D Structure") (ElapsedSeconds :type "Float (double-precision)") (TriggeredSeconds :type "Float (double-precision)") (InputAction :type "InputAction Object Reference" :default "/Game/Input/IA_PlayerMove.IA_PlayerMove"))
  (bind (_returnvalue_roll _returnvalue_pitch _returnvalue_yaw) (`KismetMathLibrary.BreakRotator` (`self.GetControlRotation`)))
  (bind (_returnvalue_x _returnvalue_y) (`KismetMathLibrary.BreakVector2D` (`KismetMathLibrary.Normal2D` ActionValue)))
  (bind _returnvalue (`KismetMathLibrary.MakeRotator` 0.0 0.0 _returnvalue_yaw))
  ; 플레이어 움직임
  (:`Triggered`
    (bind _iscanmove (`self.IsCanMove`))
    (if _iscanmove
      (set `self.IsMove` true)
      (`self.AddMovementInput` (`KismetMathLibrary.GetRightVector` _returnvalue) _returnvalue_x)
      (`self.AddMovementInput` (`KismetMathLibrary.GetForwardVector` _returnvalue) _returnvalue_y)))
  (:`Canceled`
    (set `self.IsMove` false :!label _label))
  (:`Completed`
    (goto _label)))

(event `EnhancedInput|/Game/Input/IA_BPlayerAction`
  (params (ActionValue :type Boolean) (ElapsedSeconds :type "Float (double-precision)") (TriggeredSeconds :type "Float (double-precision)") (InputAction :type "InputAction Object Reference" :default "/Game/Input/IA_BPlayerAction.IA_BPlayerAction"))
  (bind _charactermovement (`self.CharacterMovement`))
  ; 달리기 기능
  (:`Triggered`
    (if (or (`self.IsAttack`) (not (`self.IsMove`)))
      _
      (elif ActionValue
        (bind _iscanusestamina (`self.IsCanUseStamina` 1.0 :!label _label_2))
        (if _iscanusestamina
          (bind _output_get (set `self.MoveSpeed` 600.0))
          (set `CharacterMovementComponent.MaxWalkSpeed` _output_get _charactermovement)
          (else
            (bind _output_get_2 (set `self.MoveSpeed` 400.0 :!label _label_3))
            (set `CharacterMovementComponent.MaxWalkSpeed` _output_get_2 _charactermovement)))
        (else
          (goto _label_3)))))
  (:`Ongoing`
    (goto _label_2))
  (:`Completed`
    (goto _label_3)))

(event `EnhancedInput|/Game/Input/IA_PlayerLook`
  (params (ActionValue :type "Vector2D Structure") (ElapsedSeconds :type "Float (double-precision)") (TriggeredSeconds :type "Float (double-precision)") (InputAction :type "InputAction Object Reference" :default "/Game/Input/IA_PlayerLook.IA_PlayerLook"))
  (bind (_returnvalue_x _returnvalue_y) (`KismetMathLibrary.BreakVector2D` (* ActionValue (`self.MouseSensitivity`))))
  ; 시야
  (:`Triggered`
    (`self.AddControllerYawInput` _returnvalue_x)
    (`self.AddControllerPitchInput` _returnvalue_y)))

(event `EnhancedInput|/Game/Input/IA_PlayerAttack`
  (params (ActionValue :type Boolean) (ElapsedSeconds :type "Float (double-precision)") (TriggeredSeconds :type "Float (double-precision)") (InputAction :type "InputAction Object Reference" :default "/Game/Input/IA_PlayerAttack.IA_PlayerAttack"))
  ; 공격기능
  (:`Triggered`
    (`self.NotBlock`)
    (bind _iscanusestamina (`self.IsCanUseStamina` 30.0))
    (if (and _iscanusestamina (not (`self.IsAttack`)))
      (`self.Attacking`)
      (set `self.IsAttack` true))))

(event `OnDie`
  (bind _mesh (`self.Mesh`))
  ; 죽을때 처리
  (`Controller.UnPossess` (`GameplayStatics.GetPlayerController` 0))
  (`PrimitiveComponent.SetCollisionProfileName` _mesh "Ragdoll" false)
  (`PrimitiveComponent.SetSimulatePhysics` _mesh true)
  (message `/Game/Interface/BPI_Respawner.ReSpawnPlayer` (`GameplayStatics.GetGameMode`))
  (`KismetSystemLibrary.Delay` 3.0)
  (`self.K2_DestroyActor`))

(event `NotBlock`
  ; 방어기능 비활성화
  (set `self.IsBlock` false)
  (`PrimitiveComponent.SetCollisionEnabled` (`self.ShieldCollision`) "NoCollision"))

(event `EnhancedInput|/Game/Input/IA_PlayerBlock`
  (params (ActionValue :type Boolean) (ElapsedSeconds :type "Float (double-precision)") (TriggeredSeconds :type "Float (double-precision)") (InputAction :type "InputAction Object Reference" :default "/Game/Input/IA_PlayerBlock.IA_PlayerBlock"))
  ; 방어기능 활성화
  (:`Triggered`
    (if (and (not (`self.IsAttack`)) (not (<= (`self.Stamina`) 0.0)))
      (set `self.IsBlock` ActionValue)
      (`PrimitiveComponent.SetCollisionEnabled` (`self.ShieldCollision`) "QueryOnly"))))

(event `/Game/Interface/BPI_PlayerData.EndAttack`
  (`PrimitiveComponent.SetCollisionEnabled` (`self.SwordCollision`) "NoCollision"))

(event `/Game/Interface/BPI_PlayerData.EndAttackMotion`
  (set `self.IsAttack` false))

(event `self.SwordCollision.OnComponentBeginOverlap`
  (params (OverlappedComponent :type "PrimitiveComponent Object Reference") (OtherActor :type "Actor Object Reference") (OtherComp :type "PrimitiveComponent Object Reference") (OtherBodyIndex :type Integer) (bFromSweep :type Boolean) (SweepResult :type "HitResult Structure (by ref)"))
  ; 검 콜라이더와 충돌한 액터에 대미지 주기
  (if (not (== OtherActor self))
    (`GameplayStatics.ApplyDamage` OtherActor (`self.Power`))))

(event `/Game/Interface/BPI_PlayerData.StartAttack`
  (`PrimitiveComponent.SetCollisionEnabled` (`self.SwordCollision`) "QueryOnly"))

(event `self.ReceiveTick`
  (params (DeltaSeconds :type "Float (single-precision)"))
  (`self.StaminaUp` DeltaSeconds)
  (`self.LookAtTarget`))

(event `self.ReceiveAnyDamage`
  (params (Damage :type "Float (single-precision)") (DamageType :type "DamageType Object Reference") (InstigatedBy :type "Controller Object Reference") (DamageCauser :type "Actor Object Reference"))
  ; 데미지 받을때 처리 함수
  (if (`self.IsBlock`)
    (bind _iscanusestamina (`self.IsCanUseStamina` Damage))
    (if (not _iscanusestamina)
      (`self.NotBlock`)
      (set `self.Hp` (- (`self.Hp`) (- Damage (`self.Stamina`))))
      (set `self.Stamina` 0.0)
      (`self.HpChange` (stale _output_get) (`self.MaxHp`) :!label _label_4)
      (if (<= (stale _output_get) 0.0)
        (`self.OnDie`)))
    (else
      (bind _output_get (set `self.Hp` (- (`self.Hp`) Damage)))
      (goto _label_4))))

(event `StaminaUp`
  (params (DeltaTime :type "Float (double-precision)"))
  (bind _stamina (`self.Stamina`))
  ; 스테미나 자연회복
  (if (or (`self.IsAttack`) (`self.IsBlock`))
    _
    (elif (> (`self.MaxStamina`) _stamina)
      (set `self.Stamina` (+ (* DeltaTime 10.0) _stamina))
      (`self.StaminaChange` (`self.Stamina`) (`self.MaxStamina`)))))

(event `EnhancedInput|/Game/Input/IA_PlayerInputKey`
  (params (ActionValue :type Boolean) (ElapsedSeconds :type "Float (double-precision)") (TriggeredSeconds :type "Float (double-precision)") (InputAction :type "InputAction Object Reference" :default "/Game/Input/IA_PlayerInputKey.IA_PlayerInputKey"))
  ; 락온 기능 활성화/비활성화 기능
  (:`Triggered`
    (`PrimitiveComponent.SetCollisionEnabled` (`self.Sphere`) "QueryOnly")
    (bind _output_get (set `self.IslockTarget` (not (`self.IslockTarget`))))
    (bind _output_get_2 (set `self.IslookTarget` _output_get))
    (if _output_get_2
      (`self.GetTarget`))))

(event `self.Sphere.OnComponentBeginOverlap`
  (params (OverlappedComponent :type "PrimitiveComponent Object Reference") (OtherActor :type "Actor Object Reference") (OtherComp :type "PrimitiveComponent Object Reference") (OtherBodyIndex :type Integer) (bFromSweep :type Boolean) (SweepResult :type "HitResult Structure (by ref)"))
  ; 락온범위 안으로 들어온 액터 추가
  (if (!= OtherActor self)
    (`KismetArrayLibrary.Array_Add` (`self.InSphereActorList`) OtherActor)))

(event `self.Sphere.OnComponentEndOverlap`
  (params (OverlappedComponent :type "PrimitiveComponent Object Reference") (OtherActor :type "Actor Object Reference") (OtherComp :type "PrimitiveComponent Object Reference") (OtherBodyIndex :type Integer))
  ; 락온범위 밖으로 나간 액터 삭제
  (`KismetArrayLibrary.Array_RemoveItem` (`self.InSphereActorList`) OtherActor))

(event `LookAtTarget`
  (bind _target (`self.Target`))
  (bind _returnvalue (`KismetMathLibrary.FindLookAtRotation` (`self.K2_GetActorLocation`) (`self.K2_GetActorLocation` _target)))
  ; Target 액터방향으로 시점 고정
  (if (`self.IslookTarget`)
    (`/Engine/EditorBlueprintResources/StandardMacros.IsValid` _target
      (:`Is Valid`
        (`self.K2_SetActorRotation` _returnvalue)
        (`Controller.SetControlRotation` (`GameplayStatics.GetPlayerController` 0) _returnvalue)))))

(event `GetTarget`
  (bind _output (`|GetArrayItem` (`self.InSphereActorList`)))
  ; 범위내에 가장 가까운 액터를 Target으로 지정
  (`/Engine/EditorBlueprintResources/StandardMacros.IsValid` _output
    (:`Is Valid`
      (set `self.MinLength` (`KismetMathLibrary.VSize` (- (`self.K2_GetActorLocation` _output) (`self.K2_GetActorLocation`))))
      (set `self.Target` _output)
      (for _array_element (`self.InSphereActorList`)
        (bind _returnvalue (`KismetMathLibrary.VSize` (- (`self.K2_GetActorLocation` _array_element) (`self.K2_GetActorLocation`))))
        (if (< _returnvalue (`self.MinLength`))
          (set `self.Target` _array_element)
          (set `self.MinLength` _returnvalue))))
    (:`Is Not Valid`
      (set `self.Target` null))))

(fn `IsAlive`
  (returns (IsAlive :type Boolean))
  (return (> (`self.Hp`) 0.0)))

(fn `IsCanMove`
  (returns (IsCanMove :type Boolean))
  (return (not (or (`self.IsAttack`) (`self.IsBlock`)))))

(fn `IsCanUseStamina`
  (params (UseStamina :type "Float (double-precision)"))
  (returns (IsCanUseStamina :type Boolean))
  (locals (NewLocalVar :type Boolean :default false))
  (bind _returnvalue (- (`self.Stamina`) UseStamina))
  (set `local.NewLocalVar` false)
  (if (> _returnvalue 0.0)
    (bind _output_get (set `self.Stamina` _returnvalue))
    (`self.StaminaChange` _output_get (`self.MaxStamina`))
    (set `local.NewLocalVar` true))
  (return (`local.NewLocalVar`)))

(fn `UserConstructionScript`
  (set `CharacterMovementComponent.MaxWalkSpeed` (`self.MoveSpeed`) (`self.CharacterMovement`)))